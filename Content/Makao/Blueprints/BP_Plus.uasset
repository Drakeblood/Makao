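; BP_Plus is a touchable plus button in Makao that adds to the player's bet on one of four colours.
; On touch, it checks that PlayerCash in GM_Makao covers CashToBet, then adds that amount to the ACColoursCounter total matching its Type.
; The Yellow type feeds GreenCash, and PlayerCash always drops by a hardcoded 10 rather than by CashToBet.
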(event OnInputTouchBegin(StaticMesh)
  (params (FingerIndex :type ETouchIndex%20Enum :default "Touch1") (TouchedComponent :type Primitive%20Component%20Object%20Reference))
  (bind _returnvalue (Game|GetGameMode))
  (bind _returnvalue_2 (Game|GetGameMode))
  (bind _asgm_makao (Utilities|Casting|CastToGM_Makao _returnvalue))
  (bind _asgm_makao_2 (Utilities|Casting|CastToGM_Makao _returnvalue_2))
  (bind _ac_colourscounter (Variables|/Game/Makao/GameModes/GM_Makao.GM_Makao_C|GetAC_ColoursCounter _asgm_makao_2))
  (if (>= (Variables|/Game/Makao/GameModes/GM_Makao.GM_Makao_C|GetPlayerCash (.AsGM%20Makao (Utilities|Casting|CastToGM_Makao (Game|GetGameMode)))) (Variables|Default|GetCashToBet))
    (switch name (Variables|Default|GetType)
      (:Blue
        (Variables|/Game/Makao/Components/AC_ColoursCounter.AC_ColoursCounter_C|SetBlueCash _ac_colourscounter (+ (Variables|/Game/Makao/Components/AC_ColoursCounter.AC_ColoursCounter_C|GetBlueCash _ac_colourscounter) (Variables|Default|GetCashToBet))))
      (:Yellow
        (Variables|/Game/Makao/Components/AC_ColoursCounter.AC_ColoursCounter_C|SetGreenCash _ac_colourscounter (+ (Variables|/Game/Makao/Components/AC_ColoursCounter.AC_ColoursCounter_C|GetGreenCash _ac_colourscounter) (Variables|Default|GetCashToBet))))
      (:Purple
        (Variables|/Game/Makao/Components/AC_ColoursCounter.AC_ColoursCounter_C|SetPurpleCash _ac_colourscounter (+ (Variables|/Game/Makao/Components/AC_ColoursCounter.AC_ColoursCounter_C|GetPurpleCash _ac_colourscounter) (Variables|Default|GetCashToBet))))
      (:Orange
        (Variables|/Game/Makao/Components/AC_ColoursCounter.AC_ColoursCounter_C|SetOrangeCash _ac_colourscounter (+ (Variables|/Game/Makao/Components/AC_ColoursCounter.AC_ColoursCounter_C|GetOrangeCash _ac_colourscounter) (Variables|Default|GetCashToBet)))))
    (Variables|/Game/Makao/GameModes/GM_Makao.GM_Makao_C|SetPlayerCash _asgm_makao (- (Variables|/Game/Makao/GameModes/GM_Makao.GM_Makao_C|GetPlayerCash _asgm_makao) 10))))

(fn ConstructionScript)