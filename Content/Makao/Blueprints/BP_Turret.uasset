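; BP_Turret is a color-coded turret that sweeps its yaw back and forth over 90 degrees and fires bursts of bullets.
; A ping-pong timeline, started on BeginPlay when a material is set, drives rotation.
; Fire runs a looping timer that spawns BP_Bullet at the barrel, passing materials, ColorId and owner.
; DestroyTurret removes its bullets and switches BP_CubeMapElement actors of its color to a fixed ColorId before expiring.
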(event Custom|Fire
  (params (BulletCount :type Integer))
  (Variables|Default|SetShootCount BulletCount)
  (bind _returnvalue (Utilities|Time|SetTimerbyEvent (delegate Custom|FireInternal) (Variables|Default|GetShootRate) true))
  (Variables|Default|SetEventTimer _returnvalue))

(event Custom|FireInternal
  (if (> (Variables|Default|GetShootCount) 0)
    (Game|SpawnActorfromClass "/Game/Makao/Blueprints/BP_Bullet.BP_Bullet_C" (Transformation|GetWorldTransform (Variables|Default|GetBarrel)) "AlwaysSpawn" "MultiplyWithRoot" 0 (Variables|Default|GetMaterialInstance) self (Variables|Default|GetMaterialToApplyBullet) (Variables|Default|GetMaterialToApplyBulletTrail) (Variables|Default|GetColorId) 0)
    (Math|Integer|DecrementInt (Variables|Default|GetShootCount))
    (else
      (Utilities|Time|ClearandInvalidateTimerbyHandle (Variables|Default|GetEventTimer)))))

(event Custom|DestroyTurret
  (Utilities|FlowControl|Sequence
    (:then_0
      (bind _outactors (Actor|GetAllActorsOfClass "/Game/Makao/Blueprints/BP_Bullet.BP_Bullet_C"))
      (for _array_element _outactors
        (if (== (Variables|/Game/Makao/Blueprints/BP_Bullet.BP_Bullet_C|GetParentTurret _array_element) self)
          (Actor|DestroyActor _array_element))))
    (:then_1
      (bind _outactors_2 (Actor|GetAllActorsOfClass "/Game/Makao/Blueprints/BP_CubeMapElement.BP_CubeMapElement_C"))
      (for _array_element_2 _outactors_2
        (if (Utilities|Enum|Equal(Enum) (Variables|/Game/Makao/Blueprints/BP_CubeMapElement.BP_CubeMapElement_C|GetColorId _array_element_2) (Variables|Default|GetColorId))
          (Variables|/Game/Makao/Blueprints/BP_CubeMapElement.BP_CubeMapElement_C|SetColorId _array_element_2 "NewEnumerator4")))
      (Actor|SetLifeSpan 0.1))))

(event EventBeginPlay
  (if (Utilities|IsValid (Variables|Default|GetMaterialInstance))
    (Rendering|Material|SetMaterial (Variables|Default|GetTurretBodyMesh) 0 (Variables|Default|GetMaterialInstance))
    (Rendering|Material|SetMaterial (Variables|Default|GetTurretHeadMesh) 0 (Variables|Default|GetMaterialInstance))
    (Variables|Default|SetIsPlayingFromStart true)
    (bind _output_get (Variables|Default|SetStartRotation (.yaw (Variables|/Script/Engine.SceneComponent|GetRelativeRotation (Variables|Default|GetScene)))))
    (Variables|Default|SetMaxRotation (+ _output_get 9e+01))
    (Components|Timeline|PlayfromStart (Variables|Default|GetTL_RotateTurret))
    (else
      (Development|PrintString "material instance not set for turret")
      (Development|PrintString (Utilities|GetDisplayName self)))))

(fn ConstructionScript)