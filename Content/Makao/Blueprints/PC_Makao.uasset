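; Player controller for Makao that sets up the HUD and turns touch swipes into camera turns.
; On possess it caches the BP_Pawn and adds a new WBP_HUD to the viewport.
; While a touch is active, movement past a threshold calls the pawn's up/down or right/left camera turn, checking the vertical axis first.
; Each swipe fires only one turn, as the touch is deactivated once triggered.
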(event EventPossess
  (params (PossessedPawn :type Pawn%20Object%20Reference))
  (Variables|Default|SetBPPawn (.AsBP%20Pawn (Utilities|Casting|CastToBP_Pawn PossessedPawn)))
  (bind _returnvalue (UserInterface|CreateWidget "/Game/Makao/Blueprints/UI/WBP_HUD.WBP_HUD_C"))
  (UserInterface|Viewport|AddtoViewport _returnvalue 0))

(event Input|TouchEvents|InputTouch
  (params (Location :type Vector) (FingerIndex :type ETouchIndex%20Enum))
  (bind _returnvalue (Math|Vector2D|MakeVector2D (.x Location) (.y Location)))
  (:Pressed
    (Variables|Default|SetTouchStartLocation _returnvalue)
    (Variables|Default|SetTouchActive true))
  (:Released
    (Variables|Default|SetTouchActive false))
  (:Moved
    (Variables|Default|SetTouchCurrentLocation _returnvalue)
    (if (Variables|Default|GetTouchActive)
      (if (> (.y (- (Variables|Default|GetTouchStartLocation) (Variables|Default|GetTouchCurrentLocation))) (Variables|Default|GetTouchMovementTreshold))
        (Variables|Default|SetTouchActive false)
        (Default|TurnCameraUpDown (Variables|Default|GetBPPawn) false)
        (elif (< (.y (- (Variables|Default|GetTouchStartLocation) (Variables|Default|GetTouchCurrentLocation))) (* (Variables|Default|GetTouchMovementTreshold) -1.0))
          (Variables|Default|SetTouchActive false)
          (Default|TurnCameraUpDown (Variables|Default|GetBPPawn) true)
          (elif (> (.x (- (Variables|Default|GetTouchStartLocation) (Variables|Default|GetTouchCurrentLocation))) (Variables|Default|GetTouchMovementTreshold))
            (Variables|Default|SetTouchActive false)
            (Default|TurnCameraRightLeft (Variables|Default|GetBPPawn) false)
            (elif (< (.x (- (Variables|Default|GetTouchStartLocation) (Variables|Default|GetTouchCurrentLocation))) (* (Variables|Default|GetTouchMovementTreshold) -1.0))
              (Variables|Default|SetTouchActive false)
              (Default|TurnCameraRightLeft (Variables|Default|GetBPPawn) true))))))))

(fn ConstructionScript)