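; Pinball machine actor for Makao that builds up ammo and fires turrets of the matching color.
; The ball launches with random direction between two arrows and random impulse.
; Four trigger boxes reset it and start a timer: three reset or multiply Ammo, one fires matching GameMode turrets with clamped Ammo, then resets it.
; PlayWings flaps two wings repeatedly through a sped-up timeline.
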(event OnComponentBeginOverlap(Box)
  (params (OverlappedComponent :type Primitive%20Component%20Object%20Reference) (OtherActor :type Actor%20Object%20Reference) (OtherComp :type Primitive%20Component%20Object%20Reference) (OtherBodyIndex :type Integer) (bFromSweep :type Boolean) (SweepResult :type Hit%20Result%20Structure%20%28by%20ref%29))
  (CallFunction|ResetBall)
  (Variables|Default|SetAmmo 1))

(event OnComponentBeginOverlap(Box1)
  (params (OverlappedComponent :type Primitive%20Component%20Object%20Reference) (OtherActor :type Actor%20Object%20Reference) (OtherComp :type Primitive%20Component%20Object%20Reference) (OtherBodyIndex :type Integer) (bFromSweep :type Boolean) (SweepResult :type Hit%20Result%20Structure%20%28by%20ref%29))
  (CallFunction|ResetBall)
  (Variables|Default|SetAmmo (* (Variables|Default|GetAmmo) 2)))

(event OnComponentBeginOverlap(Box2)
  (params (OverlappedComponent :type Primitive%20Component%20Object%20Reference) (OtherActor :type Actor%20Object%20Reference) (OtherComp :type Primitive%20Component%20Object%20Reference) (OtherBodyIndex :type Integer) (bFromSweep :type Boolean) (SweepResult :type Hit%20Result%20Structure%20%28by%20ref%29))
  (CallFunction|ResetBall)
  (for _array_element (Variables|/Game/Makao/GameModes/GM_Makao.GM_Makao_C|GetTurrets (.AsGM%20Makao (Utilities|Casting|CastToGM_Makao (Game|GetGameMode))))
    (Utilities|IsValid _array_element
      (:Is%20Valid
        (if (== (Variables|Default|GetColor) (Utilities|String|EnumtoString (Variables|/Game/Makao/Blueprints/BP_Turret.BP_Turret_C|GetColorId _array_element)))
          (Default|Fire _array_element (Math|Integer|Clamp(Integer) (Variables|Default|GetAmmo) 5 20))
          (Development|PrintString (Utilities|String|ToString(Integer) (Variables|Default|GetAmmo)))
          (Variables|Default|SetAmmo 1))))))

(event OnComponentBeginOverlap(Box3)
  (params (OverlappedComponent :type Primitive%20Component%20Object%20Reference) (OtherActor :type Actor%20Object%20Reference) (OtherComp :type Primitive%20Component%20Object%20Reference) (OtherBodyIndex :type Integer) (bFromSweep :type Boolean) (SweepResult :type Hit%20Result%20Structure%20%28by%20ref%29))
  (CallFunction|ResetBall)
  (Variables|Default|SetAmmo (* (Variables|Default|GetAmmo) 5)))

(event Custom|PlayWings
  (params (Count :type Integer))
  (Variables|Default|SetRest Count)
  (Components|Timeline|PlayfromStart (Variables|Default|GetWingsTimeline) :!label _label)
  (bind _result (Math|Integer|DecrementInt (Variables|Default|GetRest))
    (:%20%20
      (if (Math|Conversions|ToBoolean(Integer) _result)
        (Utilities|FlowControl|Delay 1.2)
        (goto _label)))))

(event EventBeginPlay
  (Utilities|FlowControl|Delay 2.0)
  (CallFunction|FirePinBall))

(fn ConstructionScript
  (Components|Timeline|SetPlayRate (Variables|Default|GetWingsTimeline) 1e+01))

(fn FirePinBall
  (Physics|SetSimulatePhysics (Variables|Default|GetSphere) true)
  (Physics|AddImpulseatLocation (Variables|Default|GetSphere) (* (Math|Vector|GetForwardVector (Math|Rotator|Lerp(Rotator) (Math|Rotator|MakeRotfromX (Math|Vector|GetForwardVector (Variables|Default|GetArrow))) (Math|Rotator|MakeRotfromX (Math|Vector|GetForwardVector (Variables|Default|GetArrow1))) (Math|Random|RandomFloat))) (Math|Random|RandomFloatinRange (Variables|Default|GetStartUpImpulseMin) (Variables|Default|GetStartUpImpulseMax))) (Transformation|GetWorldLocation (Variables|Default|GetSphere)) "None"))

(fn ResetBall
  (Physics|SetSimulatePhysics (Variables|Default|GetSphere) false)
  (Transformation|SetWorldLocation (Variables|Default|GetSphere) (Math|Transform|TransformLocation (Transformation|GetActorTransform) "-3.000000,-53.000000,48.553733") false false)
  (Utilities|Time|SetTimerbyEvent (EventDispatchers|CreateEvent :!event FirePinBall) 1.0))