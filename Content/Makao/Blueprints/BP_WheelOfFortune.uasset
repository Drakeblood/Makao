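; BP_WheelOfFortune is a physics-driven prize wheel that spins on BeginPlay and resolves to a reward number from 1 to 4.
; TurnWheel enables physics on the Plane, applies a torque, then polls angular velocity every second until it nearly stops.
; It then disables physics and prints GetReward, which picks the arrow component pointing near world up, falling back to the highest forward Z.
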(event Custom|TurnWheel
  (Physics|SetSimulatePhysics (Variables|Default|GetPlane) true)
  (Class|PrimitiveComponent|AddTorqueinRadians (Variables|Default|GetPlane) "0.000000,10000.000000,0.000000" "None" false)
  (Utilities|FlowControl|Delay 1.0 :!label _label)
  (if (> (Math|Vector|VectorLength (Physics|GetPhysicsAngularVelocityinDegrees (Variables|Default|GetPlane) "None")) 1.0)
    (goto _label)
    (else
      (Physics|SetSimulatePhysics (Variables|Default|GetPlane) false)
      (Development|PrintString (Utilities|String|ToString(Integer) (CallFunction|GetReward))))))

(event EventBeginPlay
  (CallFunction|TurnWheel))

(fn ConstructionScript)

(fn GetReward
  (if (Utilities|Operators|EqualEqual (Math|Vector|GetForwardVector (Variables|Default|GetArrow1)) "0.000000,0.000000,1.000000" 0.5)
    (return 1)
    (elif (Utilities|Operators|EqualEqual (Math|Vector|GetForwardVector (Variables|Default|GetArrow2)) "0.000000,0.000000,1.000000" 0.5)
      (return 2)
      (elif (Utilities|Operators|EqualEqual (Math|Vector|GetForwardVector (Variables|Default|GetArrow3)) "0.000000,0.000000,1.000000" 0.5)
        (return 3)
        (elif (Utilities|Operators|EqualEqual (Math|Vector|GetForwardVector (Variables|Default|GetArrow4)) "0.000000,0.000000,1.000000" 0.5)
          (return 4)
          (else
            (return (+ (.IndexOfMaxValue (Math|Float|MaxOfFloatArray (Utilities|Array|MakeArray (.z (Math|Vector|GetForwardVector (Variables|Default|GetArrow1))) (.z (Math|Vector|GetForwardVector (Variables|Default|GetArrow2))) (.z (Math|Vector|GetForwardVector (Variables|Default|GetArrow3))) (.z (Math|Vector|GetForwardVector (Variables|Default|GetArrow4)))))) 1))))))))