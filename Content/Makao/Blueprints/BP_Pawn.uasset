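; Player pawn for the Makao game that animates the view between a default pose and two alternates, tilted or shifted sideways.
; TurnCameraUpDown rotates the Camera by timeline, while TurnCameraRightLeft slides the whole pawn to a side position precomputed in the construction script.
; Each timeline plays forward or reverse on a state change, ignoring calls while it runs or while the other view is active.
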(event Custom|TurnCameraRightLeft
  (params (Right :type Boolean))
  (if (Math|Boolean|ANDBoolean (!= Right (Variables|Default|GetRight)) (not (Audio|Components|Audio|IsPlaying (Variables|Default|GetTimelineCameraRight))) (not (Variables|Default|GetUp)))
    (bind _output_get (Variables|Default|SetRight Right))
    (if _output_get
      (bind _newtrack_0 (Timeline|TimelineCameraRight PlayFromStart)
        (:Update
          (Transformation|SetActorLocation (Math|Vector|Lerp(Vector) (Variables|Default|GetInitialPawnLocation) (Variables|Default|GetLeftSideLocation) _newtrack_0) false false)))
      (else
        (Timeline|TimelineCameraRight ReverseFromEnd)))))

(event Custom|TurnCameraUpDown
  (params (Up :type Boolean))
  (if (Math|Boolean|ANDBoolean (!= Up (Variables|Default|GetUp)) (not (Audio|Components|Audio|IsPlaying (Variables|Default|GetTimelineUpDown))) (not (Variables|Default|GetRight)))
    (bind _output_get (Variables|Default|SetUp Up))
    (if _output_get
      (bind _newtrack_0 (Timeline|TimelineUpDown PlayFromStart)
        (:Update
          (Transformation|SetRelativeRotation (Variables|Default|GetCamera) (Math|Rotator|Lerp(Rotator) "0, 0, 0" "45.000000,0.000000,0.000000" _newtrack_0) false false)))
      (else
        (Timeline|TimelineUpDown ReverseFromEnd)))))

(event EventBeginPlay)

(event Collision|EventActorBeginOverlap
  (params (OtherActor :type Actor%20Object%20Reference)))

(event EventTick
  (params (DeltaSeconds :type Float%20%28single-precision%29)))

(fn ConstructionScript
  (Variables|Default|SetInitialPawnLocation (Transformation|GetActorLocation))
  (Variables|Default|SetLeftSideLocation (+ (* (Transformation|GetActorRightVector) (Variables|Default|GetMoveLeftOffset)) (Transformation|GetActorLocation))))