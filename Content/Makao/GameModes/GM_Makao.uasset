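; Makao game mode that drives a four-colour territory battle between turrets and tracks betting odds for each colour.
; A looping timer finds every BP_Turret and fires each with a random value.
; After each shot, ACColoursCounter recounts the coloured map cubes and passes the totals to ColorTerritoryBetting.
; The odds for that turret's colour are then printed as debug text.
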(event Custom|Fire
  (bind _ac_colourscounter (Variables|Default|GetAC_ColoursCounter))
  (bind _outactors (Actor|GetAllActorsOfClass "/Game/Makao/Blueprints/BP_Turret.BP_Turret_C"))
  (bind _output_get (Variables|Default|SetTurrets _outactors))
  (for _array_element _output_get
    (Default|Fire _array_element (Math|Random|RandomInteger 20))
    (Default|CountColoursOfMapCubes _ac_colourscounter)
    (Class|ColorTerritoryBettingComponent|SetAllBlockCounts (Variables|Default|GetColorTerritoryBetting) (Default|GetBlueValue _ac_colourscounter) (Default|GetOrangeValue _ac_colourscounter) (Default|GetGreenValue _ac_colourscounter) (Default|GetPurpleValue _ac_colourscounter))
    (switch Utilities|FlowControl|Switch|SwitchonE_ColorId (Variables|/Game/Makao/Blueprints/BP_Turret.BP_Turret_C|GetColorId _array_element)
      (:NewEnumerator0
        (Development|PrintString (Utilities|String|ToString(Text) (Utilities|Text|FormatText "Color {Color} 
odds {odds}" (Utilities|String|EnumtoString (Variables|/Game/Makao/Blueprints/BP_Turret.BP_Turret_C|GetColorId _array_element)) (Class|ColorTerritoryBettingComponent|GetOdds (Variables|Default|GetColorTerritoryBetting) "Blue")))))
      (:NewEnumerator1
        (Development|PrintString (Utilities|String|ToString(Text) (Utilities|Text|FormatText "Color {Color} 
odds {odds}" (Utilities|String|EnumtoString (Variables|/Game/Makao/Blueprints/BP_Turret.BP_Turret_C|GetColorId _array_element)) (Class|ColorTerritoryBettingComponent|GetOdds (Variables|Default|GetColorTerritoryBetting) "Green")))))
      (:NewEnumerator2
        (Development|PrintString (Utilities|String|ToString(Text) (Utilities|Text|FormatText "Color {Color} 
odds {odds}" (Utilities|String|EnumtoString (Variables|/Game/Makao/Blueprints/BP_Turret.BP_Turret_C|GetColorId _array_element)) (Class|ColorTerritoryBettingComponent|GetOdds (Variables|Default|GetColorTerritoryBetting) "Purple")))))
      (:NewEnumerator3
        (Development|PrintString (Utilities|String|ToString(Text) (Utilities|Text|FormatText "Color {Color} 
odds {odds}" (Utilities|String|EnumtoString (Variables|/Game/Makao/Blueprints/BP_Turret.BP_Turret_C|GetColorId _array_element)) (Class|ColorTerritoryBettingComponent|GetOdds (Variables|Default|GetColorTerritoryBetting) "Orange"))))))))

(event EventBeginPlay
  (Utilities|Time|SetTimerbyEvent (delegate Custom|Fire) 2.0 true))

(fn ConstructionScript)