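; Actor component that tallies how many map cubes in the level are currently each of four colours: blue, green, purple and orange.
; Every tick it resets the counters, scans all BP_CubeMapElement actors and increments the counter matching each cube's ColorId.
; It prints the four totals on screen each frame and exposes them through getter functions.
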(event Custom|CountColoursOfMapCubes
  (Variables|Default|SetBlueCount 0)
  (Variables|Default|SetGreenCount 0)
  (Variables|Default|SetPurpleCount 0)
  (Variables|Default|SetOrangeCount 0)
  (bind _outactors (Actor|GetAllActorsOfClass "/Game/Makao/Blueprints/BP_CubeMapElement.BP_CubeMapElement_C"))
  (for _array_element _outactors
    (switch Utilities|FlowControl|Switch|SwitchonE_ColorId (Variables|/Game/Makao/Blueprints/BP_CubeMapElement.BP_CubeMapElement_C|GetColorId _array_element)
      (:NewEnumerator0
        (Math|Integer|IncrementInt (Variables|Default|GetBlueCount)))
      (:NewEnumerator1
        (Math|Integer|IncrementInt (Variables|Default|GetGreenCount)))
      (:NewEnumerator2
        (Math|Integer|IncrementInt (Variables|Default|GetPurpleCount)))
      (:NewEnumerator3
        (Math|Integer|IncrementInt (Variables|Default|GetOrangeCount))))))

(event EventTick
  (params (DeltaSeconds :type Float%20%28single-precision%29))
  (CallFunction|CountColoursOfMapCubes)
  (Development|PrintString (Utilities|String|ToString(Text) (Utilities|Text|FormatText "Blue {BlueCount} 
Green {GreenCount} 
Purple {PurpleCount} 
Orange {OrangeCount}" (Variables|Default|GetBlueCount) (Variables|Default|GetGreenCount) (Variables|Default|GetPurpleCount) (Variables|Default|GetOrangeCount)))))

(fn GetBlueCount
  (return (Variables|Default|GetBlueCount)))

(fn GetGreenCount
  (return (Variables|Default|GetGreenCount)))

(fn GetPurpleCount
  (return (Variables|Default|GetPurpleCount)))

(fn GetOrangeCount
  (return (Variables|Default|GetOrangeCount)))